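; Base VR pawn that handles health, death and timed revival.
; Health lives in a resource component: damage subtracts from it while alive, and its update event refreshes a normalized WBP_Health widget bar.
; Reaching the minimum runs death logic, shows death text and starts a delay timer.
; Revival restores full health and hides the text, with InitDeath and InitRevival called for state-specific setup.
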(event EventBeginPlay
  (CallFunction|InitHealth)
  (CallFunction|UpdateWidgetHealth))

(event OnMinVal(BP_ResourceBaseComponent)
  (CallFunction|Death))

(event OnUpdateVal(BP_ResourceBaseComponent)
  (CallFunction|UpdateWidgetHealth))

(event Game|Damage|EventAnyDamage
  (params (Damage :type Float%20%28single-precision%29) (DamageType :type Damage%20Type%20Object%20Reference) (InstigatedBy :type Controller%20Object%20Reference) (DamageCauser :type Actor%20Object%20Reference))
  (if (not (Class|PawnVRBase|IsDeath))
    (Default|AddVal (Variables|Default|GetBP_ResourceBaseComponent) (* Damage -1.0))))

(fn ConstructionScript)

(fn InitHealth
  (Default|SetVal (Variables|Default|GetBP_ResourceBaseComponent) 1e+02))

(fn Revival
  (Class|PawnVRBase|InitRevival)
  (Default|SetVal (Variables|Default|GetBP_ResourceBaseComponent) 1e+02)
  (Rendering|SetVisibility (Variables|Default|GetText_Death) false false))

(fn Death
  (Class|PawnVRBase|InitDeath)
  (Rendering|SetVisibility (Variables|Default|GetText_Death) true false)
  (CallFunction|ActivateTimerRevival))

(fn UpdateWidgetHealth
  (bind _bp_resourcebasecomponent (Variables|Default|GetBP_ResourceBaseComponent))
  (bind (_val _minval _maxval) (Default|GetVal _bp_resourcebasecomponent))
  (bind _aswbp_health (Utilities|Casting|CastToWBP_Health (UserInterface|GetUserWidgetObject (Variables|Default|GetWidgetHealth))))
  (Default|SetPercent _aswbp_health (Math|Float|Clamp(Float) (/ (- _val _minval) (- _maxval _minval)))))

(fn ActivateTimerRevival
  (bind _returnvalue (Utilities|Time|SetTimerbyEvent (EventDispatchers|CreateEvent :!event Revival) (Variables|Revival|GetTimeDelayRevival)))
  (Variables|Revival|SetTimerRevival _returnvalue))