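; BP_ResourceBaseComponent is a base component for a numeric resource bounded by a minimum and maximum value.
; SetVal clamps the value to that range and fires the OnUpdateVal dispatcher.
; AddVal applies a delta through SetVal, then fires OnMinVal or OnMaxVal if a limit is reached, a check SetVal alone skips.
; GetVal returns the current value with both bounds.
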(fn SetVal
  (params (Val :type Float%20%28single-precision%29))
  (Variables|Default|SetVal (Math|Float|Clamp(Float) Val (Variables|Default|GetMinVal) (Variables|Default|GetMaxVal)))
  (Default|CallOnUpdateVal))

(fn CheckMinMaxVal
  (if (<= (Variables|Default|GetVal) (Variables|Default|GetMinVal))
    (Default|CallOnMinVal)
    (elif (>= (Variables|Default|GetVal) (Variables|Default|GetMaxVal))
      (Default|CallOnMaxVal))))

(fn AddVal
  (params (AddVal :type Float%20%28single-precision%29))
  (CallFunction|SetVal (+ AddVal (Variables|Default|GetVal)))
  (CallFunction|CheckMinMaxVal))

(fn GetVal
  (return (Variables|Default|GetVal) (Variables|Default|GetMinVal) (Variables|Default|GetMaxVal)))