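; BP_Test_Damage is a test actor that takes damage, flashes red and destroys itself when its resource runs out.
; A resource component, set to full at BeginPlay, is reduced by each AnyDamage event, which also briefly swaps the sphere's material to red.
; The component's OnMinVal event destroys the actor after a short delay.
; The construction script applies the default material to the sphere.
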(event OnMinVal(BP_ResourceBaseComponent)
  (Utilities|FlowControl|Delay 0.2)
  (Actor|DestroyActor))

(event Game|Damage|EventAnyDamage
  (params (Damage :type Float%20%28single-precision%29) (DamageType :type Damage%20Type%20Object%20Reference) (InstigatedBy :type Controller%20Object%20Reference) (DamageCauser :type Actor%20Object%20Reference))
  (Default|AddVal (Variables|Default|GetBP_ResourceBaseComponent) (* Damage -1.0))
  (Rendering|Material|SetMaterial (Variables|Default|GetSphere) 0 "/Game/Assets/Materials/BAse/Color/M_Color_Red.M_Color_Red")
  (Utilities|FlowControl|Delay 0.1)
  (Rendering|Material|SetMaterial (Variables|Default|GetSphere) 0 (Variables|Default|GetDefaultMaterial)))

(event EventBeginPlay
  (Default|SetVal (Variables|Default|GetBP_ResourceBaseComponent) 1e+02))

(fn ConstructionScript
  (Rendering|Material|SetMaterial (Variables|Default|GetSphere) 0 (Variables|Default|GetDefaultMaterial)))