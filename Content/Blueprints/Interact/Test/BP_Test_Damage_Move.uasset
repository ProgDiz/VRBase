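; BP_Test_Damage_Move is a test enemy that roams and shoots at the VR player.
; After a short startup delay it caches the player pawn, starts a looping timer with a randomized interval, and glides endlessly between random MovePoints using MoveComponentTo.
; Shot fires WeaponShot toward the player's AimSphere only when a WorldStatic line trace finds no obstruction.
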(event Custom|MoveTo
  (bind _returnvalue (CallFunction|GetRandomTarget))
  (Utilities|IsValid _returnvalue
    (:Is%20Valid
      (Components|MoveComponentTo (Variables|Default|GetDefaultSceneRoot) (Transformation|GetActorLocation _returnvalue) "0, 0, 0" false false 5.0 false)
      (CallFunction|Moveto))))

(event EventBeginPlay
  (|CallParentFunction)
  (Utilities|FlowControl|Delay 0.5)
  (CallFunction|InitEnemy)
  (CallFunction|ActiavteTimerShot)
  (CallFunction|Moveto))

(fn ConstructionScript
  (|CallParentFunction))

(fn Shot
  (Variables|Default|GetEnemy
    (:then
      (if (not (CallFunction|CheckVisibilityEnemy))
        (Class|WeaponShotComponent|Shot (Variables|Default|GetWeaponShot) (Transformation|GetActorLocation) (Math|Vector|Normalize (- (Transformation|GetWorldLocation (Variables|/Game/Blueprints/Pawns/BP_PawnVRBase.BP_PawnVRBase_C|GetAimSphere (Variables|Default|GetEnemy))) (Transformation|GetActorLocation))))))
    (:else)))

(fn InitEnemy
  (bind _asbp_pawn_vrbase (Utilities|Casting|CastToBP_PawnVRBase (Game|Player|GetPlayerPawn 0)))
  (Variables|Default|SetEnemy _asbp_pawn_vrbase))

(fn ActiavteTimerShot
  (Utilities|Time|SetTimerbyEvent (EventDispatchers|CreateEvent :!event Shot) (Math|Random|RandomFloatinRange 1.0 2.0) true))

(fn GetRandomTarget
  (bind _movepoints (Variables|Default|GetMovePoints))
  (if (> (Utilities|Array|Length _movepoints) 0)
    (return (.OutItem (Utilities|Array|Random _movepoints)))))

(fn CheckVisibilityEnemy
  (bind _enemy (Variables|Default|GetEnemy)
    (:then
      (bind _returnvalue (Collision|LineTraceForObjects (Transformation|GetActorLocation) (Transformation|GetWorldLocation (Variables|/Game/Blueprints/Pawns/BP_PawnVRBase.BP_PawnVRBase_C|GetAimSphere _enemy)) (Utilities|Array|MakeArray "ObjectTypeQuery1") false 0 "None"))
      (return _returnvalue))
    (:else)))